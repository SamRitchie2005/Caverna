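; Turn manager for a two-team, turn-based combat game that spawns the characters, rotates turns and ends the match.
; Once the map's trace check passes, it spawns GameInstance-defined characters at random map-validated spots and shuffles their order.
; State flags route Enhanced Input to the active character, free camera or heal-other ally selection.
; Character deaths update the roster, and a wiped-out team stores the winner in the GameInstance and opens the end level.
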(event Custom|CharacterDeath
  (params (Character :type BP%20Character%20Object%20Reference))
  (bind _returnvalue (Game|GetGameInstance))
  ;[0.15 0.15 0.15 0.5] Handle character death and game ending
  (Variables|Default|SetisCharacterTemp (Utilities|Array|Get(acopy) (Variables|Default|GetCharacters) (Variables|Default|GetTurnIndex)))
  (Utilities|Array|RemoveItem (Variables|Default|GetCharacters) Character)
  (if (== Character (Variables|Default|GetisCharacterTemp))
    (CallFunction|EndTurn)
    (CallFunction|MoveSet)
    (elif (Variables|/Game/BP_Character.BP_Character_C|Getdrowned Character)
      (Math|Integer|DecrementInt (Variables|Default|GetTurnIndex)
        (:%20%20
          _))))
  (Variables|Default|Setteam1Num 0)
  (Variables|Default|Setteam2Num 0)
  (for _array_element (Variables|Default|GetCharacters)
    (if (== (Variables|/Game/BP_Character.BP_Character_C|GetTeam _array_element) 1)
      (Math|Integer|IncrementInt (Variables|Default|Getteam1Num))
      (else
        (Math|Integer|IncrementInt (Variables|Default|Getteam2Num)))))
  (if (== (Variables|Default|Getteam1Num) 0)
    (bind _asgame_instance_1 (Utilities|Casting|CastToGameInstance1 _returnvalue))
    (Variables|/Game/GameInstance1.GameInstance1_C|SetWhoWin _asgame_instance_1 2)
    (Game|OpenLevel(byName) "L_End" :!label _label)
    (elif (== (Variables|Default|Getteam2Num) 0)
      (bind _asgame_instance_1_2 (Utilities|Casting|CastToGameInstance1 _returnvalue))
      (Variables|/Game/GameInstance1.GameInstance1_C|SetWhoWin _asgame_instance_1_2 1)
      (goto _label))))

(event Custom|CreateProjectile
  (params (Projectile :type BP%20Projectile%20Generic%20Object%20Reference))
  ;[0.15 0.15 0.15 0.5] Add projectiles to projectile list
  (Utilities|Array|Add (Variables|Default|GetProjectiles) Projectile))

(event Custom|DestroyProjectile
  ;[0.15 0.15 0.15 0.5] Remove Finished projectiles from list
  (for _array_element (Variables|Default|GetProjectiles)
    (if (Variables|/Game/WeaponsItems/Generics/BP_ProjectileGeneric.BP_ProjectileGeneric_C|GetFinished _array_element)
      (Utilities|Array|RemoveItem (Variables|Default|GetProjectiles) _array_element))))

(event Custom|SpawnCharacters
  ;[0.15 0.15 0.15 0.5] Spawn Characters
  (for _array_element (Variables|Default|GetCharacterSpawnArray)
    (bind _spawnloc (CallFunction|FSpawnChecker))
    (bind _returnvalue (Game|SpawnActorfromClass "/Game/BP_Character.BP_Character_C" (Math|Transform|MakeTransform (Math|Vector|MakeVector 7.3e+02 (.x _spawnloc) (+ (.y _spawnloc) 95.0)) "0, 0, 0" "1.000000,1.000000,1.000000") "AlwaysSpawn" "MultiplyWithRoot" 0 0))
    (Default|InitialInit _returnvalue self (Variables|Default|Getmap) (.team _array_element) (Variables|Default|Getitems) (.class _array_element))
    (Utilities|Array|Add (Variables|Default|GetCharacters) _returnvalue))
  (for _array_element_2 (Variables|Default|GetCharacters)
    (for _array_element_3 (Variables|Default|GetCharacters)
      (if (!= _array_element_3 _array_element_2)
        (if (== (Variables|/Game/BP_Character.BP_Character_C|GetTeam _array_element_3) (Variables|/Game/BP_Character.BP_Character_C|GetTeam _array_element_2))
          (Default|InitTeammates _array_element_2 _array_element_3))))))

(event Custom|HealOtherActivate
  (params (HealOtherItem :type BP%20Heal%20Other%20Item%20Object%20Reference))
  ;[0.15 0.15 0.15 0.5] Heal Other Item Handle
  (Variables|Default|SetHeal%20Other%20Item HealOtherItem)
  (Variables|Default|SetHealOtherActive true)
  (Variables|Default|SetTurnActive false))

(event Custom|HealOtherDeactivate
  ;[0.15 0.15 0.15 0.5] Heal Other Item Handle
  (Variables|Default|SetHealOtherActive false)
  (Variables|Default|SetTurnActive true))

(event Custom|ActivateCharacter
  ;[0 0 0] Activate Character turn
  (Default|InitTurn (Utilities|Array|Get(acopy) (Variables|Default|GetCharacters) (Variables|Default|GetTurnIndex)) self))

(event Custom|EndTurn
  ;[0 0 0] Ends the Turn and Rotates Through Registered Characters
  (Variables|Default|SetTurnActive false)
  (bind _result (Math|Integer|IncrementInt (Variables|Default|GetTurnIndex))
    (:%20%20
      (Viewport|RemoveAllWidgets)
      (if (> _result (Utilities|Array|LastIndex (Variables|Default|GetCharacters)))
        (Variables|Default|SetTurnIndex 0))
      (CallFunction|ActivateCharacter))))

(event Custom|ItemSelect
  (params (item :type Integer))
  ;[0.15 0.15 0.15 0.5] Input item select from Inventory
  (Variables|Default|SetTurnActive true)
  (Default|ItemSelected (Utilities|Array|Get(acopy) (Variables|Default|GetCharacters) (Variables|Default|GetTurnIndex)) item))

(event Custom|InitCheck
  (bind _returnvalue (Game|GetPlayerController 0))
  (bind _returnvalue_2 (PlayerController|LocalPlayerSubsystems|GetEnhancedInputLocalPlayerSubsystem _returnvalue))
  ;[0.15 0.15 0.15 0.5] Init
  (bind _testresult (Default|TraceTest (stale EventBeginPlay _output_get)))
  (if _testresult
    (Utilities|FlowControl|Sequence
      (:then_0
        (Utilities|Time|ClearandInvalidateTimerbyHandle (stale EventBeginPlay _returnvalue_2)))
      (:then_1
        (bind _outactors (Actor|GetAllActorsOfClass "/Game/WeaponsItems/Generics/BP_ItemGeneric.BP_ItemGeneric_C"))
        (Variables|Default|Setitems _outactors)
        (bind _asgame_instance_1 (Utilities|Casting|CastToGameInstance1 (Game|GetGameInstance))
          (:then
            (Variables|Default|SetCharacterSpawnArray (Variables|/Game/GameInstance1.GameInstance1_C|GetCharacterInfo _asgame_instance_1)))
          (:CastFailed
            _))
        (Utilities|IsValid _returnvalue_2
          (:Is%20Valid
            (Input|AddMappingContext _returnvalue_2 "/Game/Inputs/IMC_Default.IMC_Default" 0 "(bIgnoreAllPressedKeysUntilRelease=True,bForceImmediately=False,bNotifyUserSettings=False)")
            (CallFunction|SpawnCharacters)
            (CallFunction|FSortCharacterArray)
            (CallFunction|FBindtoEvents)
            (CallFunction|ActivateCharacter)
            (Variables|/Script/Engine.PlayerController|SetbShowMouseCursor (Game|GetPlayerController 0) false)
            (Audio|PlaySound2D "/Game/SFX/hitslab-battle-warrior-fighting-drums-430819.hitslab-battle-warrior-fighting-drums-430819" 0.2 1.0 0.0 0 0)))))))

(event Input|EnhancedActionEvents|EnhancedInputActionIA_SetDestination_Click
  (params (ActionValue :type Boolean) (ElapsedSeconds :type Float%20%28double-precision%29) (TriggeredSeconds :type Float%20%28double-precision%29) (InputAction :type Input%20Action%20Object%20Reference :default "/Game/TopDown/Input/Actions/IA_SetDestination_Click.IA_SetDestination_Click"))
  ;[0.15 0.15 0.15 0.5] Input Use Item
  (:Completed
    (if (Variables|Default|GetTurnActive)
      (bind _returnvalue (Class|WidgetLayoutLibrary|GetMousePositiononViewport))
      (Default|Fireproto (Utilities|Array|Get(acopy) (Variables|Default|GetCharacters) (Variables|Default|GetTurnIndex)) (Math|Conversions|ToVector(Vector2D) (- _returnvalue (Class|SlateBlueprintLibrary|ScreentoViewport (/ (Viewport|GetViewportSize) "(X=2.000000,Y=2.000000)")))) (Variables|Default|Getmap)))))

(event Input|EnhancedActionEvents|EnhancedInputActionIA_jump
  (params (ActionValue :type Boolean) (ElapsedSeconds :type Float%20%28double-precision%29) (TriggeredSeconds :type Float%20%28double-precision%29) (InputAction :type Input%20Action%20Object%20Reference :default "/Game/Inputs/IA_jump.IA_jump"))
  (bind _characters (Variables|Default|GetCharacters))
  (bind _turnindex (Variables|Default|GetTurnIndex))
  (bind _output (Utilities|Array|Get(acopy) _characters _turnindex))
  ;[0.15 0.15 0.15 0.5] Input Jump
  (:Started
    (if (Variables|Default|GetTurnActive)
      (Character|Jump _output)
      (Audio|PlaySoundatLocation "/Game/SFX/SFX_Land.SFX_Land" (Transformation|GetActorLocation _output) "0, 0, 0" 1.0 1.0 0.0 0 0 0 0))))

(event Input|EnhancedActionEvents|EnhancedInputActionIA_move
  (params (ActionValue :type Float%20%28double-precision%29) (ElapsedSeconds :type Float%20%28double-precision%29) (TriggeredSeconds :type Float%20%28double-precision%29) (InputAction :type Input%20Action%20Object%20Reference :default "/Game/Inputs/IA_move.IA_move"))
  ;[0.15 0.15 0.15 0.5] Input Move
  (if (Variables|Default|GetTurnActive)
    (Default|Moveproto (Utilities|Array|Get(acopy) (Variables|Default|GetCharacters) (Variables|Default|GetTurnIndex)) ActionValue)))

(event Input|EnhancedActionEvents|EnhancedInputActionIA_CameraLookTrigger
  (params (ActionValue :type Boolean) (ElapsedSeconds :type Float%20%28double-precision%29) (TriggeredSeconds :type Float%20%28double-precision%29) (InputAction :type Input%20Action%20Object%20Reference :default "/Game/Inputs/IA_CameraLookTrigger.IA_CameraLookTrigger"))
  (bind _returnvalue (Game|GetPlayerController 0))
  (bind _returnvalue_2 (Pawn|GetViewTarget _returnvalue))
  ;[0.15 0.15 0.15 0.5] trigger Free cam look
  (:Triggered
    (if (Variables|Default|GetTurnActive)
      (Variables|Default|SetTurnActive false)
      (Variables|Default|SetCameraMove true)))
  (:Canceled
    (if (Variables|Default|GetCameraMove) :!label _label
      (Variables|Default|SetTurnActive true)
      (Variables|Default|SetCameraMove false)
      (if (Utilities|DoesObjectImplementInterface _returnvalue_2 "/Game/interfaces/BP_CameraInterface.BP_CameraInterface_C")
        (bind _camera (Class|BPCameraInterface|GetCamera(Message) _returnvalue_2))
        (Transformation|SetRelativeLocation _camera "0, 0, 0" false false))))
  (:Completed
    (goto _label)))

(event Input|EnhancedActionEvents|EnhancedInputActionIA_MoveCamera
  (params (ActionValue :type Vector%202D%20Structure) (ElapsedSeconds :type Float%20%28double-precision%29) (TriggeredSeconds :type Float%20%28double-precision%29) (InputAction :type Input%20Action%20Object%20Reference :default "/Game/TopDown/Input/Actions/IA_MoveCamera.IA_MoveCamera"))
  (bind _returnvalue (Game|GetPlayerController 0))
  (bind _returnvalue_2 (Pawn|GetViewTarget _returnvalue))
  ;[0.15 0.15 0.15 0.5] Move camera when in free cam mode
  (if (Variables|Default|GetCameraMove)
    (if (Utilities|DoesObjectImplementInterface _returnvalue_2 "/Game/interfaces/BP_CameraInterface.BP_CameraInterface_C")
      (bind _camera (Class|BPCameraInterface|GetCamera(Message) _returnvalue_2))
      (Transformation|AddLocalOffset _camera (Math|Vector|MakeVector 0.0 (* (.y ActionValue) 1e+01) (* (.x ActionValue) 1e+01)) false false))))

(event Input|EnhancedActionEvents|EnhancedInputActionIA_HealOtherSelect
  (params (ActionValue :type Boolean) (ElapsedSeconds :type Float%20%28double-precision%29) (TriggeredSeconds :type Float%20%28double-precision%29) (InputAction :type Input%20Action%20Object%20Reference :default "/Game/WeaponsItems/HealOther/IA_HealOtherSelect.IA_HealOtherSelect"))
  ;[0.15 0.15 0.15 0.5] Heal Other Item Handle
  (:Started
    (if (Variables|Default|GetHealOtherActive)
      (Class|HealOtherInterface|AllySelect(Message) (Variables|Default|GetHeal%20Other%20Item)))))

(event Input|EnhancedActionEvents|EnhancedInputActionIA_HealOtherCycle
  (params (ActionValue :type Float%20%28double-precision%29) (ElapsedSeconds :type Float%20%28double-precision%29) (TriggeredSeconds :type Float%20%28double-precision%29) (InputAction :type Input%20Action%20Object%20Reference :default "/Game/WeaponsItems/HealOther/IA_HealOtherCycle.IA_HealOtherCycle"))
  ;[0.15 0.15 0.15 0.5] Heal Other Item Handle
  (:Started
    (if (Variables|Default|GetHealOtherActive)
      (Class|HealOtherInterface|AllyCycle(Message) (Variables|Default|GetHeal%20Other%20Item) (Math|Float|Truncate ActionValue)))))

(event Input|EnhancedActionEvents|EnhancedInputActionIA_InventoryEnter
  (params (ActionValue :type Boolean) (ElapsedSeconds :type Float%20%28double-precision%29) (TriggeredSeconds :type Float%20%28double-precision%29) (InputAction :type Input%20Action%20Object%20Reference :default "/Game/Inputs/IA_InventoryEnter.IA_InventoryEnter"))
  ;[0.15 0.15 0.15 0.5] Input enter inventory
  (if (Variables|Default|GetTurnActive)
    (Variables|Default|SetTurnActive false)
    (Default|EnterInventory (Utilities|Array|Get(acopy) (Variables|Default|GetCharacters) (Variables|Default|GetTurnIndex)))))

(event EventBeginPlay
  ;[0.15 0.15 0.15 0.5] Init
  (Variables|Default|SetTraceTest false)
  (bind _returnvalue (Actor|GetActorOfClass "/Game/Map/BP_Map.BP_Map_C"))
  (bind _output_get (Variables|Default|Setmap _returnvalue))
  (bind _returnvalue_2 (Utilities|Time|SetTimerbyEvent (delegate Custom|InitCheck) 0.1 true)))

(event EventMoveSet
  ;[0.15 0.15 0.15 0.5] Set next character turn as active
  (Variables|Default|SetTurnActive true)
  (Game|Player|SetViewTargetwithBlend (Game|GetPlayerController 0) (Utilities|Array|Get(acopy) (Variables|Default|GetCharacters) (Variables|Default|GetTurnIndex)) 0.0 "VTBlend_Linear" 0.0 false))

(fn ConstructionScript)

(fn FSortCharacterArray
  (while (Utilities|Array|IsValidIndex (Variables|Default|GetCharacters))
    (bind _output_get (LocalVariables|SetCharRef (.OutItem (Utilities|Array|Random (Variables|Default|GetCharacters)))))
    (Utilities|Array|Add (LocalVariables|GetOrderedCharacterArray) _output_get)
    (Utilities|Array|RemoveItem (Variables|Default|GetCharacters) _output_get))
  (Variables|Default|SetCharacters (LocalVariables|GetOrderedCharacterArray))
  (return))

(fn FBindtoEvents
  (for _array_element (Variables|Default|GetCharacters)
    (EventDispatchers|BindEventtoEDEndTurn _array_element (EventDispatchers|CreateEvent :!event Custom|EndTurn)))
  (return))

(fn FSpawnChecker
  (Variables|Default|SetspawnCheck true)
  (while (Variables|Default|GetspawnCheck)
    (bind _output_get (Variables|Default|SetSpawnAttempt (Math|Vector2D|MakeVector2D (Math|Random|RandomFloatinRange -1.64e+03 2.9e+03) (Math|Random|RandomFloatinRange 3e+03 7.5e+03))))
    (bind (_x _y _true) (Default|SpawnTrace (Variables|Default|Getmap) (.x _output_get) (.y _output_get)))
    (Variables|Default|SetSpawnAttempt (Math|Vector2D|MakeVector2D _x _y))
    (if _true
      (Variables|Default|SetspawnCheck false)))
  (return (Variables|Default|GetSpawnAttempt)))

(fn RetrieveItems
  (bind _characters (Variables|Default|GetCharacters))
  (bind _turnindex (Variables|Default|GetTurnIndex))
  (bind _output (Utilities|Array|Get(acopy) _characters _turnindex))
  (return (Variables|/Game/BP_Character.BP_Character_C|GetInventory _output) (Variables|/Game/BP_Character.BP_Character_C|Getcurrent%20item%20index _output)))