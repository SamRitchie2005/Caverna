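; BP_Border is a map actor that procedurally generates a border wall mesh at BeginPlay with Geometry Script.
; It builds a subdivided rectangle and boolean-subtracts an offset second rectangle created on a compute mesh.
; The result is distorted with Perlin noise and linearly extruded in a fixed direction for thickness, and the component receives the wall material.
; Construction script and Tick are empty.
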(event Collision|EventActorBeginOverlap
  (params (OtherActor :type Actor%20Object%20Reference)))

(event EventTick
  (params (DeltaSeconds :type Float%20%28single-precision%29)))

(event EventBeginPlay
  ;[0.15 0.15 0.15 0.5] Dynamically generate border wall at runtime
  (bind _returnvalue (DynamicMeshComponent|GetDynamicMesh (Variables|DynamicMeshActor|GetDynamicMeshComponent)))
  (bind _output_get (Variables|Default|SetTarget%20Mesh _returnvalue))
  (bind _returnvalue_2 (Class|GeometryScriptLibraryMeshPrimitiveFunctions|AppendRectangleXY :TargetMesh _output_get :DimensionX 2e+02 :DimensionY 2e+02 :StepsWidth 100 :StepsHeight 100 :Debug 0))
  (bind _returnvalue_3 (DynamicMeshActor|AllocateComputeMesh))
  (bind _returnvalue_4 (Class|GeometryScriptLibraryMeshPrimitiveFunctions|AppendRectangleXY :TargetMesh _returnvalue_3 :DimensionX 2e+02 :Debug 0))
  (bind _returnvalue_5 (GeometryScript|Booleans|ApplyMeshBoolean :TargetMesh _returnvalue_2 :ToolMesh _returnvalue_4 :ToolTransform (Math|Transform|MakeTransform "50.000000,0.000000,0.000000") :Operation "Subtract" :Options (Utilities|Struct|MakeGeometryScriptMeshBooleanOptions false true) :Debug 0))
  (bind _returnvalue_6 (Class|GeometryScriptLibraryMeshDeformFunctions|ApplyPerlinNoisetoMesh :TargetMesh _returnvalue_5 :Options (Utilities|Struct|MakeGeometryScriptPerlinNoiseOptions "(Magnitude=5.000000,Frequency=0.250000,FrequencyShift=(X=0.000000,Y=0.000000,Z=0.000000),RandomSeed=0)" false "FullMeshSelection") :Debug 0))
  (bind _returnvalue_7 (Class|GeometryScriptLibraryMeshModelingFunctions|ApplyMeshLinearExtrudeFaces :TargetMesh _returnvalue_6 :Options (Utilities|Struct|MakeGeometryScriptMeshLinearExtrudeOptions 1e+01 "FixedDirection") :Debug 0))
  (GeometryScript|Scene|SetComponentMaterialList (Variables|DynamicMeshActor|GetDynamicMeshComponent) (Utilities|Array|MakeArray "/Game/Map/M_WallMaterial.M_WallMaterial") 0)
  (Variables|Default|SetTarget%20Mesh _returnvalue_7))

(fn ConstructionScript)