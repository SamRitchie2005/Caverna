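; BP_MapBorder is a procedurally generated dynamic mesh actor that, by its name, forms a map border wall.
; On mesh rebuild, Geometry Script creates a finely subdivided rectangle and boolean-subtracts an offset second rectangle from it.
; Perlin noise then displaces the result, and a fixed-direction linear extrude gives it thickness.
; The wall material is applied both on BeginPlay and after each rebuild.
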(event Collision|EventActorBeginOverlap
  (params (OtherActor :type Actor%20Object%20Reference)))

(event EventTick
  (params (DeltaSeconds :type Float%20%28single-precision%29)))

(event Events|EventOnRebuildGeneratedMesh
  (params (TargetMesh :type Dynamic%20Mesh%20Object%20Reference))
  (bind _output_get (Variables|Default|SetTarget%20Mesh TargetMesh))
  (bind _returnvalue (Class|GeometryScriptLibraryMeshPrimitiveFunctions|AppendRectangleXY :TargetMesh _output_get :DimensionX 2e+02 :DimensionY 2e+02 :StepsWidth 100 :StepsHeight 100 :Debug 0))
  (bind _returnvalue_2 (DynamicMeshActor|AllocateComputeMesh))
  (bind _returnvalue_3 (Class|GeometryScriptLibraryMeshPrimitiveFunctions|AppendRectangleXY :TargetMesh _returnvalue_2 :DimensionX 2e+02 :Debug 0))
  (bind _returnvalue_4 (GeometryScript|Booleans|ApplyMeshBoolean :TargetMesh _returnvalue :ToolMesh _returnvalue_3 :ToolTransform (Math|Transform|MakeTransform "50.000000,0.000000,0.000000") :Operation "Subtract" :Options (Utilities|Struct|MakeGeometryScriptMeshBooleanOptions false true) :Debug 0))
  (bind _returnvalue_5 (Class|GeometryScriptLibraryMeshDeformFunctions|ApplyPerlinNoisetoMesh :TargetMesh _returnvalue_4 :Options (Utilities|Struct|MakeGeometryScriptPerlinNoiseOptions "(Magnitude=5.000000,Frequency=0.250000,FrequencyShift=(X=0.000000,Y=0.000000,Z=0.000000),RandomSeed=0)" false "FullMeshSelection") :Debug 0))
  (bind _returnvalue_6 (Class|GeometryScriptLibraryMeshModelingFunctions|ApplyMeshLinearExtrudeFaces :TargetMesh _returnvalue_5 :Options (Utilities|Struct|MakeGeometryScriptMeshLinearExtrudeOptions 1e+01 "FixedDirection") :Debug 0))
  (GeometryScript|Scene|SetComponentMaterialList (Variables|DynamicMeshActor|GetDynamicMeshComponent) (Utilities|Array|MakeArray "/Game/Map/M_WallMaterial.M_WallMaterial") 0)
  (Variables|Default|SetTarget%20Mesh _returnvalue_6))

(event EventBeginPlay
  (GeometryScript|Scene|SetComponentMaterialList (Variables|DynamicMeshActor|GetDynamicMeshComponent) (Utilities|Array|MakeArray "/Game/Map/M_WallMaterial.M_WallMaterial") 0)
  (Variables|Default|SetTarget%20Mesh (stale Events|EventOnRebuildGeneratedMesh _returnvalue_6)))

(fn ConstructionScript)