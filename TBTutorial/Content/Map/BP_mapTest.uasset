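; Test map actor that uses Geometry Script to generate a randomly seeded, destructible terrain mesh.
; BeginPlay builds a subdivided rectangle, displaces it with Perlin noise, plane-cuts it, extrudes what remains, then applies collision and the map material.
; Explosion subtracts a size-scaled cylinder at the target's local position through a mesh boolean, then refreshes collision.
; OnRebuildGeneratedMesh re-enters the build chain after the seed and reset steps.
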(event EventExplosion
  (params (target :type Vector :default "0, 0, 0") (Size :type Float%20%28double-precision%29))
  (bind _returnvalue (DynamicMeshActor|AllocateComputeMesh))
  (bind _returnvalue_2 (GeometryScript|Primitives|AppendCylinder :TargetMesh _returnvalue :Radius (/ Size 2.0) :RadialSteps 24 :Origin "Center" :Debug 0))
  (Variables|Default|Setdamage%20Mesh_0 _returnvalue_2)
  (bind _returnvalue_3 (GeometryScript|Booleans|ApplyMeshBoolean :TargetMesh (Variables|Default|GetTarget%20Mesh) :ToolMesh (Variables|Default|Getdamage%20Mesh_0) :ToolTransform (Math|Transform|MakeTransform (Math|Transform|InverseTransformLocation (Transformation|GetWorldTransform (Variables|DynamicMeshActor|GetDynamicMeshComponent)) target) "0, 0, 0" "1.000000,1.000000,1.000000") :Operation "Subtract" :Options (Utilities|Struct|MakeGeometryScriptMeshBooleanOptions false true) :Debug 0))
  (Class|GeometryScriptLibraryCollisionFunctions|SetDynamicMeshCollisionfromMesh :FromDynamicMesh _returnvalue_3 :ToDynamicMeshComponent (Variables|DynamicMeshActor|GetDynamicMeshComponent) :Debug 0))

(event EventBeginPlay
  (Variables|Default|Set%20Seed (Math|Random|RandomInteger 1000000))
  (bind _returnvalue (DynamicMeshComponent|GetDynamicMesh (Variables|DynamicMeshActor|GetDynamicMeshComponent)))
  (bind _returnvalue_2 (DynamicMesh|Reset _returnvalue))
  (bind _output_get (Variables|Default|SetTarget%20Mesh _returnvalue_2))
  (bind _returnvalue_3 (Class|GeometryScriptLibraryMeshPrimitiveFunctions|AppendRectangleXY :TargetMesh _output_get :StepsWidth 100 :StepsHeight 100 :Debug 0))
  (bind _returnvalue_4 (Class|GeometryScriptLibraryMeshDeformFunctions|ApplyPerlinNoisetoMesh :TargetMesh _returnvalue_3 :Options (Utilities|Struct|MakeGeometryScriptPerlinNoiseOptions (Utilities|Struct|MakeGeometryScriptPerlinNoiseLayerOptions 5.0 0.25 "0.000000,0.000000,0.000000" (Variables|Default|Get%20Seed)) true "FullMeshSelection") :Debug 0))
  (bind _returnvalue_5 (Class|GeometryScriptLibraryMeshBooleanFunctions|ApplyMeshPlaneCut :TargetMesh _returnvalue_4 :Options (Utilities|Struct|MakeGeometryScriptMeshPlaneCutOptions false -1) :Debug 0))
  (bind _returnvalue_6 (Class|GeometryScriptLibraryMeshModelingFunctions|ApplyMeshLinearExtrudeFaces :TargetMesh _returnvalue_5 :Options (Utilities|Struct|MakeGeometryScriptMeshLinearExtrudeOptions 1e+01 "FixedDirection") :Debug 0))
  (bind _returnvalue_7 (Class|GeometryScriptLibraryCollisionFunctions|SetDynamicMeshCollisionfromMesh :FromDynamicMesh _returnvalue_6 :ToDynamicMeshComponent (Variables|DynamicMeshActor|GetDynamicMeshComponent) :Debug 0))
  (GeometryScript|Scene|SetComponentMaterialList (Variables|DynamicMeshActor|GetDynamicMeshComponent) (Utilities|Array|MakeArray "/Game/Map/M_MapMaterial.M_MapMaterial") 0)
  (Variables|Default|SetTarget%20Mesh _returnvalue_7))

(event Events|EventOnRebuildGeneratedMesh
  (params (TargetMesh :type Dynamic%20Mesh%20Object%20Reference))
  (bind _output_get (Variables|Default|SetTarget%20Mesh (stale EventBeginPlay _returnvalue_2)))
  (bind _returnvalue (Class|GeometryScriptLibraryMeshPrimitiveFunctions|AppendRectangleXY :TargetMesh _output_get :StepsWidth 100 :StepsHeight 100 :Debug 0))
  (bind _returnvalue_2 (Class|GeometryScriptLibraryMeshDeformFunctions|ApplyPerlinNoisetoMesh :TargetMesh _returnvalue :Options (Utilities|Struct|MakeGeometryScriptPerlinNoiseOptions (Utilities|Struct|MakeGeometryScriptPerlinNoiseLayerOptions 5.0 0.25 "0.000000,0.000000,0.000000" (Variables|Default|Get%20Seed)) true "FullMeshSelection") :Debug 0))
  (bind _returnvalue_3 (Class|GeometryScriptLibraryMeshBooleanFunctions|ApplyMeshPlaneCut :TargetMesh _returnvalue_2 :Options (Utilities|Struct|MakeGeometryScriptMeshPlaneCutOptions false -1) :Debug 0))
  (bind _returnvalue_4 (Class|GeometryScriptLibraryMeshModelingFunctions|ApplyMeshLinearExtrudeFaces :TargetMesh _returnvalue_3 :Options (Utilities|Struct|MakeGeometryScriptMeshLinearExtrudeOptions 1e+01 "FixedDirection") :Debug 0))
  (bind _returnvalue_5 (Class|GeometryScriptLibraryCollisionFunctions|SetDynamicMeshCollisionfromMesh :FromDynamicMesh _returnvalue_4 :ToDynamicMeshComponent (Variables|DynamicMeshActor|GetDynamicMeshComponent) :Debug 0))
  (GeometryScript|Scene|SetComponentMaterialList (Variables|DynamicMeshActor|GetDynamicMeshComponent) (Utilities|Array|MakeArray "/Game/Map/M_MapMaterial.M_MapMaterial") 0)
  (Variables|Default|SetTarget%20Mesh _returnvalue_5))

(fn ConstructionScript)