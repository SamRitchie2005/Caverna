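; BP_Water is a water volume that builds its surface at runtime and notifies characters and projectiles that fall into it.
; On BeginPlay, Geometry Script generates a subdivided plane in the DynamicMeshComponent, displaces it with Perlin noise, extrudes it and applies the water material.
; Box overlaps send drown messages to actors of exactly BP_Character class or to any BP_ProjectileGeneric subclass.
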(event OnComponentBeginOverlap(Box)
  (params (OverlappedComponent :type Primitive%20Component%20Object%20Reference) (OtherActor :type Actor%20Object%20Reference) (OtherComp :type Primitive%20Component%20Object%20Reference) (OtherBodyIndex :type Integer) (bFromSweep :type Boolean) (SweepResult :type Hit%20Result%20Structure%20%28by%20ref%29))
  (bind _returnvalue (Utilities|GetClass OtherActor))
  (if (== _returnvalue "/Game/BP_Character.BP_Character_C")
    (Class|BPInterfacetest|Drown(Message) OtherActor)
    (elif (Utilities|ClassIsChildOf _returnvalue "/Game/WeaponsItems/Generics/BP_ProjectileGeneric.BP_ProjectileGeneric_C")
      (Class|BPInterfacetest|ProjectileDrown(Message) OtherActor))))

(event Collision|EventActorBeginOverlap
  (params (OtherActor :type Actor%20Object%20Reference)))

(event EventTick
  (params (DeltaSeconds :type Float%20%28single-precision%29)))

(event EventBeginPlay
  (bind _returnvalue (DynamicMeshComponent|GetDynamicMesh (Variables|DynamicMeshActor|GetDynamicMeshComponent)))
  (bind _output_get (Variables|Default|SetTarget%20Mesh _returnvalue))
  (bind _returnvalue_2 (Class|GeometryScriptLibraryMeshPrimitiveFunctions|AppendRectangleXY :TargetMesh _output_get :DimensionX 2e+02 :DimensionY 2e+02 :StepsWidth 100 :StepsHeight 100 :Debug 0))
  (bind _returnvalue_3 (Class|GeometryScriptLibraryMeshDeformFunctions|ApplyPerlinNoisetoMesh :TargetMesh _returnvalue_2 :Options (Utilities|Struct|MakeGeometryScriptPerlinNoiseOptions "(Magnitude=5.000000,Frequency=0.250000,FrequencyShift=(X=0.000000,Y=0.000000,Z=0.000000),RandomSeed=0)" false "FullMeshSelection") :Debug 0))
  (Class|GeometryScriptLibraryMeshModelingFunctions|ApplyMeshLinearExtrudeFaces :TargetMesh _returnvalue_3 :Options (Utilities|Struct|MakeGeometryScriptMeshLinearExtrudeOptions 1e+01 "FixedDirection") :Debug 0)
  (GeometryScript|Scene|SetComponentMaterialList (Variables|DynamicMeshActor|GetDynamicMeshComponent) (Utilities|Array|MakeArray "/Game/Map/M_WaterMaterial.M_WaterMaterial") 0))

(fn ConstructionScript)