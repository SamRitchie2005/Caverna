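; Playable team character for a turn-based game, with one of five classes setting its inventory, health, movement and mesh, and team setting its materials.
; Turn events handle camera, indicator and HUD; movement and item use check IsTurn.
; Items are picked through an inventory widget and fired by calling UseItem on that class's existing level actor.
; Damage and healing share an invincibility timer; death or drowning explodes, purges teammates' references and notifies the Manager.
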(event Custom|InitTurn
  (params (Manager :type BP%20Turn%20Manager%20Object%20Reference))
  ;[0.3438 0.3438 0.3438] commands the Turn Manager to Ready Itself
  (Variables|Default|SetManager Manager)
  (CallFunction|InitTurnComponents true))

(event Custom|InitTurnComponents
  (params (IsTurn :type Boolean))
  ;[0.8125 0.8125 0.8125] Init Nav Blocking Volume, Is-Active-Indicator, Camera, and UI
  (Collision|SetCollisionEnabled (Variables|Default|GetNavBlockingVolume) (select IsTurn "NoCollision" "NoCollision"))
  (Rendering|SetVisibility (Variables|Default|GetIsTurnIndicator) IsTurn false)
  (Game|Player|SetViewTargetwithBlend (Game|GetPlayerController 0) self 0.5 "VTBlend_Linear" 0.0 false)
  (Variables|Default|SetCanUseItem true)
  (bind _returnvalue (UserInterface|CreateWidget "/Game/UI/UI_inGame.UI_inGame_C"))
  (bind _output_get (Variables|Default|SetGameUI _returnvalue))
  (UserInterface|Viewport|AddtoViewport _output_get 0))

(event Custom|MeshSet
  (bind _mesh (Variables|Character|GetMesh))
  (bind _mesh_2 (Variables|Character|GetMesh))
  (bind _mesh_3 (Variables|Character|GetMesh))
  (bind _mesh_4 (Variables|Character|GetMesh))
  (bind _mesh_5 (Variables|Character|GetMesh))
  ;[0 0 0 0.5] Class Initialisation
  ;;[0.15 0.15 0.15 0.5] Initialise character mesh from Class
  (switch Utilities|FlowControl|Switch|SwitchonClassName (Variables|Default|GetClass)
    (:NewEnumerator2
      (Components|SkeletalMesh|SetSkeletalMeshAsset _mesh_3 "/Game/Classes/characters/Soldier/SKM_Soldier.SKM_Soldier")
      (Components|SkeletalMesh|SetAnimInstanceClass _mesh_3 "/Game/Classes/characters/Soldier/ABP_Soldier.ABP_Soldier_C"))
    (:NewEnumerator3
      (Components|SkeletalMesh|SetSkeletalMeshAsset _mesh "/Game/Classes/characters/Tank/SKM_Tank.SKM_Tank")
      (Components|SkeletalMesh|SetAnimInstanceClass _mesh "/Game/Classes/characters/Tank/ABP_Tank.ABP_Tank_C"))
    (:NewEnumerator4
      (Components|SkeletalMesh|SetSkeletalMeshAsset _mesh_4 "/Game/Classes/characters/vanguard/SKM_Vanguard.SKM_Vanguard")
      (Components|SkeletalMesh|SetAnimInstanceClass _mesh_4 "/Game/Classes/characters/vanguard/ABP_Vanguard.ABP_Vanguard_C"))
    (:NewEnumerator5
      (Components|SkeletalMesh|SetSkeletalMeshAsset _mesh_2 "/Game/Classes/characters/Healer/SKM_Healer.SKM_Healer")
      (Components|SkeletalMesh|SetAnimInstanceClass _mesh_2 "/Game/Classes/characters/Healer/ABP_Healer.ABP_Healer_C"))
    (:NewEnumerator6
      (Components|SkeletalMesh|SetSkeletalMeshAsset _mesh_5 "/Game/Classes/characters/Demo/SKM_Demo.SKM_Demo")
      (Components|SkeletalMesh|SetAnimInstanceClass _mesh_5 "/Game/Classes/characters/Demo/ABP_Demo.ABP_Demo_C"))))

(event Custom|ItemSet
  (bind _manager (Variables|Default|GetManager))
  (bind _classes (Variables|/Game/BP_TurnManager.BP_TurnManager_C|GetClasses _manager))
  ;[0 0 0 0.5] Class Initialisation
  ;;[0.15 0.15 0.15 0.5] Initialise Item Inventory from Class
  (switch Utilities|FlowControl|Switch|SwitchonClassName (Variables|Default|GetClass)
    (:NewEnumerator2
      (Variables|Default|SetInventory (Utilities|Struct|BreakSoldier (.soldier _classes))))
    (:NewEnumerator3
      (Variables|Default|SetInventory (Utilities|Struct|BreakTank (.tank _classes))))
    (:NewEnumerator4
      (Variables|Default|SetInventory (Utilities|Struct|BreakVanguard (.vanguard _classes))))
    (:NewEnumerator5
      (Variables|Default|SetInventory (Utilities|Struct|BreakHealer (.healer _classes))))
    (:NewEnumerator6
      (Variables|Default|SetInventory (Utilities|Struct|BreakBuilder (.builder _classes))))))

(event Custom|HealthSet
  (bind _bp_health (Variables|Default|GetBP_Health))
  (bind _charactermovement (Variables|Character|GetCharacterMovement))
  (bind _charactermovement_2 (Variables|Character|GetCharacterMovement))
  ;[0 0 0 0.5] Class Initialisation
  ;;[0.15 0.15 0.15 0.5] Initialise Character stats from Class
  (switch Utilities|FlowControl|Switch|SwitchonClassName (Variables|Default|GetClass)
    (:NewEnumerator2
      (Default|SetMaxHealth _bp_health 1e+02)
      (Variables|/Script/Engine.CharacterMovementComponent|SetJumpZVelocity _charactermovement 3.5e+02)
      (Variables|/Script/Engine.CharacterMovementComponent|SetMaxWalkSpeed _charactermovement_2 5e+02))
    (:NewEnumerator3
      (Default|SetMaxHealth _bp_health 1.5e+02)
      (Variables|/Script/Engine.CharacterMovementComponent|SetJumpZVelocity _charactermovement 2e+02)
      (Variables|/Script/Engine.CharacterMovementComponent|SetMaxWalkSpeed _charactermovement_2 3e+02))
    (:NewEnumerator4
      (Default|SetMaxHealth _bp_health 1e+02)
      (Variables|/Script/Engine.CharacterMovementComponent|SetJumpZVelocity _charactermovement 6e+02)
      (Variables|/Script/Engine.CharacterMovementComponent|SetMaxWalkSpeed _charactermovement_2 8e+02))
    (:NewEnumerator5
      (Default|SetMaxHealth _bp_health 75.0)
      (Variables|/Script/Engine.CharacterMovementComponent|SetJumpZVelocity _charactermovement 4.5e+02)
      (Variables|/Script/Engine.CharacterMovementComponent|SetMaxWalkSpeed _charactermovement_2 675.0))
    (:NewEnumerator6
      (Default|SetMaxHealth _bp_health 125.0)
      (Variables|/Script/Engine.CharacterMovementComponent|SetJumpZVelocity _charactermovement 525.0)
      (Variables|/Script/Engine.CharacterMovementComponent|SetMaxWalkSpeed _charactermovement_2 725.0))))

(event Custom|iframetimer2
  ;[0.15 0.15 0.15 0.5] Healing
  (Variables|Default|Setinvincible false))

(event Custom|IframeTimer
  ;[0.15 0.15 0.15 0.5] Take Damage
  (Variables|Default|Setinvincible false))

(event Custom|Init%20teammates
  (params (mate :type BP%20Character%20Object%20Reference))
  ;[0.15 0.15 0.15 0.5] Initialise Teamates
  (Utilities|Array|Add (Variables|Default|GetTeammates) mate))

(event Custom|PurgeAlly
  (params (Character :type BP%20Character%20Object%20Reference))
  ;[0.15 0.15 0.15 0.5] Remove Ally from Ally list
  (Utilities|Array|RemoveItem (Variables|Default|GetTeammates) Character))

(event Custom|EnterInventory
  ;[0.15 0.15 0.15 0.5] Enter Inventory Menu
  (bind _returnvalue (UserInterface|CreateWidget "/Game/UI/UI_Inventory.UI_Inventory_C" (Game|GetPlayerController 0)))
  (bind _output_get (Variables|Default|SetinventoryWidget _returnvalue))
  (UserInterface|Viewport|AddtoViewport _output_get 0)
  (Variables|/Script/Engine.PlayerController|SetbShowMouseCursor (Game|GetPlayerController 0) true))

(event Custom|ItemSelected
  (params (item :type Integer))
  ;[0.15 0.15 0.15 0.5] Select Item and exit Inventory UI
  (Widget|RemovefromParent (Variables|Default|GetinventoryWidget))
  (CallFunction|ItemSwap item)
  (Variables|/Script/Engine.PlayerController|SetbShowMouseCursor (Game|GetPlayerController 0) false))

(event Custom|ItemSwap
  (params (item :type Integer))
  ;[0.15 0.15 0.15 0.5] Item switching in character and UI
  (Variables|Default|Setcurrent%20item%20index item)
  (Variables|Default|SetCurrentItem (.item (Utilities|Array|Get(acopy) (Variables|Default|GetInventory) (Variables|Default|Getcurrent%20item%20index))))
  (Variables|Default|SetcurrentAmmo (.amount (Utilities|Array|Get(acopy) (Variables|Default|GetInventory) (Variables|Default|Getcurrent%20item%20index))))
  (Widget|RemovefromParent (Variables|Default|GetGameUI))
  (bind _returnvalue (UserInterface|CreateWidget "/Game/UI/UI_inGame.UI_inGame_C"))
  (bind _output_get (Variables|Default|SetGameUI _returnvalue))
  (UserInterface|Viewport|AddtoViewport _output_get 0))

(event Custom|moveproto
  (params (param :type Float%20%28double-precision%29))
  ;[0.15 0.15 0.15 0.5] Movement
  (if (Variables|Default|GetisTurn)
    (Pawn|Input|AddMovementInput "0.000000,1.000000,0.000000" param false)))

(event Custom|EndTurn
  ;[0.7917 0.7917 0.7917] End Turn
  (CallFunction|InitTurnComponents false)
  (Variables|Default|SetisTurn true)
  (Default|CallEDEndTurn))

(event Custom|fireproto
  (params (NewParam :type Vector) (NewParam2 :type BP%20Map%20Object%20Reference))
  (bind _returnvalue (Math|Vector|Normalize NewParam))
  ;[0.15 0.15 0.15 0.5] Use item
  (if (Variables|Default|GetCanUseItem)
    (Variables|Default|Setmap NewParam2)
    (bind _result (Math|Float|NegateFloat (.y _returnvalue))
      (:%20%20
        (Variables|Default|SetAimTarget (Math|Vector|MakeVector (.z _returnvalue) (.x _returnvalue) _result))
        (if (Variables|Default|GetisTurn)
          (if (!= (Variables|Default|GetcurrentAmmo) 0)
            (Variables|Default|SetCanUseItem false)
            (if (> (Variables|Default|GetcurrentAmmo) 0)
              (bind _result_2 (Math|Integer|DecrementInt (.amount (Utilities|Array|Get(acopy) (Variables|Default|GetInventory) (Variables|Default|Getcurrent%20item%20index))))
                (:%20%20
                  (Variables|Default|SetcurrentAmmo _result_2))))
            (bind _returnvalue_2 (Actor|GetActorOfClass (Variables|Default|GetCurrentItem)))
            (Default|UseItem _returnvalue_2 self (Variables|Default|GetAimTarget) (Variables|Default|Getmap) (Variables|Default|GetManager) (Variables|Default|GetTeammates))))))))

(event Custom|Death
  ;[0.15 0.15 0.15 0.5] Character Death
  (Utilities|Time|SetTimerbyEvent (delegate Custom|DeathTimer) 1.0))

(event Custom|InitialInit
  (params (Manager :type BP%20Turn%20Manager%20Object%20Reference) (Map :type BP%20Map%20Object%20Reference) (Team :type Integer) (all%20items :type Array%20of%20BP%20Item%20Generic%20Object%20References) (Class :type ClassName%20Enum :default "NewEnumerator2"))
  (bind _isturnindicator (Variables|Default|GetIsTurnIndicator))
  (bind _current_item_index (Variables|Default|Getcurrent%20item%20index))
  (bind _mesh (Variables|Character|GetMesh))
  (bind _mesh_2 (Variables|Character|GetMesh))
  (bind _inventory (Variables|Default|GetInventory))
  (bind _output (Utilities|Array|Get(acopy) _inventory _current_item_index))
  ;[0.15 0.15 0.15 0.5] Initial initialisation
  (Variables|Default|SetManager Manager)
  (Variables|Default|Setmap Map)
  (Variables|Default|SetTeam Team)
  (Variables|Default|SetitemsAll all%20items)
  (Variables|Default|SetClass Class)
  (CallFunction|ItemSet)
  (CallFunction|HealthSet)
  (Variables|Default|SetCurrentItem (.item _output))
  (Variables|Default|SetcurrentAmmo (.amount _output))
  (CallFunction|MeshSet)
  (if (== (Variables|Default|GetTeam) 2)
    (Rendering|Material|SetMaterial _isturnindicator 0 "/Game/Framework/Materials/MI_AIHighlight.MI_AIHighlight")
    (Rendering|Material|SetMaterial _mesh_2 1 "/Game/Characters/Mannequins/Materials/Instances/Manny/MI_AIMat2.MI_AIMat2")
    (Rendering|Material|SetMaterial _mesh 0 "/Game/Characters/Mannequins/Materials/Instances/Manny/MI_AIMat.MI_AIMat")
    (else
      (Rendering|Material|SetMaterial _isturnindicator 0 "/Game/Framework/Materials/MI_PlayerHighlight.MI_PlayerHighlight")
      (Rendering|Material|SetMaterial _mesh_2 1 "/Game/Characters/Mannequins/Materials/Instances/Manny/MI_PlayerMat2.MI_PlayerMat2")
      (Rendering|Material|SetMaterial _mesh 0 "/Game/Characters/Mannequins/Materials/Instances/Manny/MI_PlayerMat.MI_PlayerMat"))))

(event Custom|DeathTimer
  (bind _returnvalue (Transformation|GetActorLocation))
  ;[0.15 0.15 0.15 0.5] Character Death
  (Collision|SetCollisionEnabled (Variables|Collision|GetCapsuleComponent) "NoCollision")
  (for _array_element (Variables|Default|GetTeammates)
    (CallFunction|PurgeAlly _array_element self))
  (Audio|PlaySoundatLocation "/Game/SFX/SFX_Explosion.SFX_Explosion" _returnvalue "0, 0, 0" 1.0 1.0 0.0 0 0 0 0)
  (Game|SpawnActorfromClass "/Game/WeaponsItems/Generics/BP_ExplsoionGeneric.BP_ExplsoionGeneric_C" (Math|Transform|MakeTransform _returnvalue "0, 0, 0" "1.000000,1.000000,1.000000") "Undefined" "MultiplyWithRoot" 0 0)
  (Default|CharacterDeath (Variables|Default|GetManager) self)
  (Actor|DestroyActor))

(event EventKnockback
  (params (Force :type Float%20%28double-precision%29) (Diraction :type Vector :default "0, 0, 0"))
  ;[0.15 0.15 0.15 0.5] Take Knockback
  (Physics|AddImpulse (Variables|Character|GetCharacterMovement) (* Force Diraction) false))

(event EventDrown
  ;[0.15 0.15 0.15 0.5] Drowning into Death
  (Variables|Default|Setdrowned true)
  (CallFunction|DeathTimer))

(event EventHeal
  (params (health :type Float%20%28double-precision%29))
  (bind _bp_health (Variables|Default|GetBP_Health))
  ;[0.15 0.15 0.15 0.5] Healing
  (Default|Heal _bp_health health)
  (if (not (Variables|Default|Getinvincible))
    (Variables|Default|Setinvincible true)
    (Class|IUI|HealthUpdate(Message) (UserInterface|GetWidget (Variables|Default|GetWidget)) (Variables|/Game/BP_Health.BP_Health_C|GetMaxHealth _bp_health) (Variables|/Game/BP_Health.BP_Health_C|GetCurrentHealth _bp_health))
    (Niagara|SpawnSystematLocation "/Game/VFX/FX_Heal.FX_Heal" (Transformation|GetActorLocation self))
    (Utilities|Time|SetTimerbyEvent (delegate Custom|iframetimer2) 0.5)))

(event EventDamage
  (params (damage :type Float%20%28double-precision%29))
  (bind _bp_health (Variables|Default|GetBP_Health))
  ;[0.15 0.15 0.15 0.5] Take Damage
  (if (not (Variables|Default|Getinvincible))
    (Default|Damage _bp_health damage)
    (Variables|Default|Setinvincible true)
    (Class|IUI|HealthUpdate(Message) (UserInterface|GetWidget (Variables|Default|GetWidget)) (Variables|/Game/BP_Health.BP_Health_C|GetMaxHealth _bp_health) (Variables|/Game/BP_Health.BP_Health_C|GetCurrentHealth _bp_health))
    (Utilities|Time|SetTimerbyEvent (delegate Custom|IframeTimer) 0.5)))

(fn ConstructionScript
  (bind _isturnindicator (Variables|Default|GetIsTurnIndicator))
  (bind _mesh (Variables|Character|GetMesh))
  (bind _mesh_2 (Variables|Character|GetMesh))
  (if (== (Variables|Default|GetTeam) 2)
    (Rendering|Material|SetMaterial _isturnindicator 0 "/Game/Framework/Materials/MI_AIHighlight.MI_AIHighlight")
    (Rendering|Material|SetMaterial _mesh_2 1 "/Game/Characters/Mannequins/Materials/Instances/Manny/MI_AIMat2.MI_AIMat2")
    (Rendering|Material|SetMaterial _mesh 0 "/Game/Characters/Mannequins/Materials/Instances/Manny/MI_AIMat.MI_AIMat")
    (else
      (Rendering|Material|SetMaterial _isturnindicator 0 "/Game/Framework/Materials/MI_PlayerHighlight.MI_PlayerHighlight")
      (Rendering|Material|SetMaterial _mesh_2 1 "/Game/Characters/Mannequins/Materials/Instances/Manny/MI_PlayerMat2.MI_PlayerMat2")
      (Rendering|Material|SetMaterial _mesh 0 "/Game/Characters/Mannequins/Materials/Instances/Manny/MI_PlayerMat.MI_PlayerMat"))))

(fn GetCamera
  (return (Variables|Default|GetCamera)))