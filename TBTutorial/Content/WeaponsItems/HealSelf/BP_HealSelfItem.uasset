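; BP_HealSelfItem is a usable item that heals the unit using it in what appears to be turn-based play.
; UseItem stores the owner, target, map and manager, plays a heal sound at the owner, then picks a heal amount by unit class, with Healers receiving more than the other classes.
; After a short timer delay, it ends the owner's turn and calls ItemEnd.
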(event Custom|CustomEvent
  (Default|EndTurn (Variables|Default|GetOwner_0))
  (CallFunction|ItemEnd))

(event EventBeginPlay
  (|CallParentFunction) ; This node is disabled and will not be called.\nDrag off pins to build functionality.
)

(event Collision|EventActorBeginOverlap
  (params (OtherActor :type Actor%20Object%20Reference))
  (|CallParentFunction OtherActor) ; This node is disabled and will not be called.\nDrag off pins to build functionality.
)

(event EventTick
  (params (DeltaSeconds :type Float%20%28single-precision%29))
  (|CallParentFunction DeltaSeconds) ; This node is disabled and will not be called.\nDrag off pins to build functionality.
)

(event EventUseItem
  (params (Owner :type BP%20Character%20Object%20Reference) (Target :type Vector :default "0, 0, 0") (Map :type BP%20Map%20Object%20Reference) (Manager :type BP%20Turn%20Manager%20Object%20Reference) (teammates :type Array%20of%20BP%20Character%20Object%20References))
  (Variables|Default|SetOwner_0 Owner)
  (Variables|Default|SetTarget Target)
  (Variables|Default|SetMap Map)
  (Variables|Default|SetManager Manager)
  (Audio|PlaySoundatLocation "/Game/SFX/SFX_Heal.SFX_Heal" (Transformation|GetActorLocation (Variables|Default|GetOwner_0)) "0, 0, 0" 1.0 1.0 0.0 0 0 0 0)
  (switch Utilities|FlowControl|Switch|SwitchonClassName (Variables|/Game/BP_Character.BP_Character_C|GetClass (Variables|Default|GetOwner_0))
    (:NewEnumerator2
      (Variables|Default|Sethealth 5e+01 :!label _label))
    (:NewEnumerator3
      (goto _label))
    (:NewEnumerator4
      (goto _label))
    (:NewEnumerator5
      (Variables|Default|Sethealth 75.0))
    (:NewEnumerator6
      (goto _label)))
  (Default|Heal (Variables|Default|GetOwner_0) (Variables|Default|Gethealth))
  (Utilities|Time|SetTimerbyEvent (delegate Custom|CustomEvent) 3.0))

(fn ConstructionScript
  (|CallParentFunction))