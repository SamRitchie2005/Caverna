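; BP_SkipGoItem is a weapon/item Blueprint that lets its user skip their go by ending their turn.
; Its UseItem event stores the owner, target, map and manager, calls EndTurn on the owner, then calls ItemEnd to finish the item.
; The target, map and manager are not otherwise used, and the default actor events are disabled.
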(event EventBeginPlay
  (|CallParentFunction) ; This node is disabled and will not be called.\nDrag off pins to build functionality.
)

(event Collision|EventActorBeginOverlap
  (params (OtherActor :type Actor%20Object%20Reference))
  (|CallParentFunction OtherActor) ; This node is disabled and will not be called.\nDrag off pins to build functionality.
)

(event EventTick
  (params (DeltaSeconds :type Float%20%28single-precision%29))
  (|CallParentFunction DeltaSeconds) ; This node is disabled and will not be called.\nDrag off pins to build functionality.
)

(event EventUseItem
  (params (Owner :type BP%20Character%20Object%20Reference) (Target :type Vector :default "0, 0, 0") (Map :type BP%20Map%20Object%20Reference) (Manager :type BP%20Turn%20Manager%20Object%20Reference) (teammates :type Array%20of%20BP%20Character%20Object%20References))
  (Variables|Default|SetOwner_0 Owner)
  (Variables|Default|SetTarget Target)
  (Variables|Default|SetMap Map)
  (Variables|Default|SetManager Manager)
  (Default|EndTurn (Variables|Default|GetOwner_0))
  (CallFunction|ItemEnd))

(fn ConstructionScript
  (|CallParentFunction))