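; Generic explosion actor, configured through Init with size, map, force, position and damage.
; On BeginPlay it notifies BP_ExplosionHandle to play FX, then a timeline grows its scale from zero to Size.
; BP_Character actors overlapped by its collision take damage and knockback away from the center.
; When the timeline finishes, it sends the Map an explosion message with a slightly enlarged size, then destroys itself.
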(event OnComponentBeginOverlap(collision)
  (params (OverlappedComponent :type Primitive%20Component%20Object%20Reference) (OtherActor :type Actor%20Object%20Reference) (OtherComp :type Primitive%20Component%20Object%20Reference) (OtherBodyIndex :type Integer) (bFromSweep :type Boolean) (SweepResult :type Hit%20Result%20Structure%20%28by%20ref%29))
  (if (== (Utilities|GetClass OtherActor) "/Game/BP_Character.BP_Character_C")
    (Class|BPInterfacetest|Knockback(Message) OtherActor (Variables|Default|GetForce) (- "" (- (Transformation|GetActorLocation) (Transformation|GetActorLocation OtherActor))))
    (Class|BPInterfacetest|Damage(Message) OtherActor (Variables|Default|GetDamage_0))))

(event Custom|Explode
  (Class|BPInterfacetest|Explosion(Message) (Variables|Default|Getmap) (Variables|Default|GetLocation) (* (Variables|Default|GetSize) 1.25))
  (Actor|DestroyActor))

(event Custom|Init
  (params (Size :type Float%20%28double-precision%29) (Map :type BP%20Map%20Object%20Reference) (Force :type Float%20%28double-precision%29) (Position :type Vector) (Damage :type Float%20%28double-precision%29))
  (Variables|Default|SetSize Size)
  (Variables|Default|Setmap Map)
  (Variables|Default|SetForce Force)
  (Variables|Default|SetLocation Position)
  (Variables|Default|SetDamage_0 Damage)
  (Collision|SetCollisionResponsetoAllChannels (Variables|Default|Getcollision) "ECR_Overlap"))

(event EventBeginPlay
  (bind _returnvalue (Actor|GetActorOfClass "/Game/VFX/BP_ExplosionHandle.BP_ExplosionHandle_C"))
  (Class|BIExplosionFX|ExplodeFx(Message) _returnvalue (Transformation|GetActorLocation))
  (bind _newtrack_0 (Timeline|Timeline Play)
    (:Update
      (Transformation|SetActorScale3D (Math|Conversions|ToVector(Float) (Math|Float|Lerp 0.0 (Variables|Default|GetSize) _newtrack_0))))
    (:Finished
      (CallFunction|Explode))))

(event Collision|EventActorBeginOverlap
  (params (OtherActor :type Actor%20Object%20Reference)))

(event EventTick
  (params (DeltaSeconds :type Float%20%28single-precision%29)))

(fn ConstructionScript)