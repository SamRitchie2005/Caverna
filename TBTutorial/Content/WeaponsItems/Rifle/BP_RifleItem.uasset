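; BP_RifleItem is a rifle item for a turn-based game, fired from its owner toward a target in the Y-Z plane.
; UseItem plays the shot sound and runs a long Camera-channel line trace that ignores the owner, with the end locked to a fixed X.
; The hit location drives a Niagara beam and spawns a generic explosion initialized with the map and damage.
; A short timer then ends the item and the owner's turn.
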(event Custom|rifleTimer
  (bind _owner_0 (Variables|Default|GetOwner_0))
  (CallFunction|ItemEnd)
  (Utilities|IsValid _owner_0
    (:Is%20Valid
      (Default|EndTurn _owner_0))))

(event EventBeginPlay
  (|CallParentFunction) ; This node is disabled and will not be called.\nDrag off pins to build functionality.
)

(event Collision|EventActorBeginOverlap
  (params (OtherActor :type Actor%20Object%20Reference))
  (|CallParentFunction OtherActor) ; This node is disabled and will not be called.\nDrag off pins to build functionality.
)

(event EventTick
  (params (DeltaSeconds :type Float%20%28single-precision%29))
  (|CallParentFunction DeltaSeconds) ; This node is disabled and will not be called.\nDrag off pins to build functionality.
)

(event EventUseItem
  (params (Owner :type BP%20Character%20Object%20Reference) (Target :type Vector :default "0, 0, 0") (Map :type BP%20Map%20Object%20Reference) (Manager :type BP%20Turn%20Manager%20Object%20Reference) (teammates :type Array%20of%20BP%20Character%20Object%20References))
  (bind _niagara (Variables|Default|GetNiagara))
  (Variables|Default|SetOwner_0 Owner)
  (Variables|Default|SetTarget Target)
  (Variables|Default|SetMap Map)
  (Variables|Default|SetManager Manager)
  (Audio|PlaySoundatLocation "/Game/SFX/SFX_GunFire.SFX_GunFire" (Transformation|GetActorLocation (Variables|Default|GetOwner_0)) "0, 0, 0" 1.0 1.0 0.0 0 0 0 0)
  (bind _outhit (Collision|LineTraceByChannel (Transformation|GetActorLocation (Variables|Default|GetOwner_0)) (Math|Vector|MakeVector 7.3e+02 (.y (+ (Transformation|GetActorLocation (Variables|Default|GetOwner_0)) (Math|Vector|MakeVector 0.0 (.y (* (Math|Vector|MakeVector 0.0 (.y (Variables|Default|GetTarget)) (.z (Variables|Default|GetTarget))) 1e+04)) (.z (* (Math|Vector|MakeVector 0.0 (.y (Variables|Default|GetTarget)) (.z (Variables|Default|GetTarget))) 1e+04))))) (.z (+ (Transformation|GetActorLocation (Variables|Default|GetOwner_0)) (Math|Vector|MakeVector 0.0 (.y (* (Math|Vector|MakeVector 0.0 (.y (Variables|Default|GetTarget)) (.z (Variables|Default|GetTarget))) 1e+04)) (.z (* (Math|Vector|MakeVector 0.0 (.y (Variables|Default|GetTarget)) (.z (Variables|Default|GetTarget))) 1e+04)))))) "TraceTypeQuery2" true (Utilities|Array|MakeArray (Variables|Default|GetOwner_0)) "None"))
  (Class|NiagaraComponent|SetNiagaraVariableVec3 (Variables|Default|GetNiagara) "Beam" (.location _outhit))
  (Transformation|SetWorldLocation _niagara (Transformation|GetActorLocation (Variables|Default|GetOwner_0)) false false)
  (Components|Activation|Activate _niagara false)
  (bind _returnvalue (Game|SpawnActorfromClass "/Game/WeaponsItems/Generics/BP_ExplsoionGeneric.BP_ExplsoionGeneric_C" (Math|Transform|MakeTransform (.location _outhit) "0, 0, 0" "1.000000,1.000000,1.000000") "Undefined" "MultiplyWithRoot" 0 0))
  (Default|Init _returnvalue 2.0 (Variables|Default|GetMap) 0.0 (.location _outhit) 6e+01)
  (Utilities|Time|SetTimerbyEvent (delegate Custom|rifleTimer) 3.0))

(fn ConstructionScript
  (|CallParentFunction))