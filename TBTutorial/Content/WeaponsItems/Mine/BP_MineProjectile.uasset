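; BP_MineProjectile is the thrown mine actor of a turn-based weapon item, exploding on a timer rather than on impact.
; InitGrenade stores the map, manager and owning item, sets damage, levels the spring arm and starts the fuse.
; GrenadeExplode returns the view, messages the item about turn end, disables and hides the projectile, then spawns BP_ExplsoionGeneric to handle the blast before calling ItemEnd.
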(event OnComponentHit(Sphere)
  (params (HitComponent :type Primitive%20Component%20Object%20Reference) (OtherActor :type Actor%20Object%20Reference) (OtherComp :type Primitive%20Component%20Object%20Reference) (NormalImpulse :type Vector :default "0, 0, 0") (Hit :type Hit%20Result%20Structure%20%28by%20ref%29)))

(event Custom|InitGrenade
  (params (map :type BP%20Map%20Object%20Reference) (Manager :type BP%20Turn%20Manager%20Object%20Reference) (Owner :type BP%20Item%20Generic%20Object%20Reference))
  (Variables|Default|SetMap map)
  (Variables|Default|SetManager Manager)
  (Variables|Default|SetowningItem Owner)
  (Variables|Default|SetDamage_0 4e+01)
  (Transformation|SetWorldRotation (Variables|Default|GetSpringArm) "0, 0, 0" false false)
  (Utilities|Time|SetTimerbyEvent (delegate Custom|GrenadeExplode) 5.0))

(event Custom|GrenadeExplode
  (bind _returnvalue (Transformation|GetActorLocation))
  (bind _sphere (Variables|Default|GetSphere))
  (Game|Player|SetViewTargetwithBlend (Game|GetPlayerController 0) 0 0.5 "VTBlend_Linear" 0.0 false)
  (Class|BPInterfacetest|MineEndTurn(Message) (Variables|Default|GetowningItem))
  (Audio|PlaySoundatLocation "/Game/SFX/SFX_Explosion.SFX_Explosion" (Transformation|GetActorLocation) "0, 0, 0" 1.0 1.0 0.0 0 0 0 0)
  (Components|Activation|Deactivate (Variables|Default|GetProjectileMovement))
  (Components|Tick|SetComponentTickEnabled _sphere false)
  (Collision|SetCollisionEnabled _sphere "NoCollision")
  (Development|SetHiddeninGame _sphere true true)
  (bind _returnvalue_2 (Game|SpawnActorfromClass "/Game/WeaponsItems/Generics/BP_ExplsoionGeneric.BP_ExplsoionGeneric_C" (Math|Transform|MakeTransform _returnvalue "0, 0, 0" "0.000000,0.000000,0.000000") "Undefined" "MultiplyWithRoot" 0 0))
  (Default|Init _returnvalue_2 (Variables|Default|GetSize) (Variables|Default|GetMap) (Variables|Default|GetForce) _returnvalue (Variables|Default|GetDamage_0))
  (Variables|Default|SetFinished true)
  (Default|ItemEnd (Variables|Default|GetowningItem)))

(event EventBeginPlay
  (|CallParentFunction) ; This node is disabled and will not be called.\nDrag off pins to build functionality.
)

(event Collision|EventActorBeginOverlap
  (params (OtherActor :type Actor%20Object%20Reference))
  (|CallParentFunction OtherActor) ; This node is disabled and will not be called.\nDrag off pins to build functionality.
)

(event EventTick
  (params (DeltaSeconds :type Float%20%28single-precision%29))
  (|CallParentFunction DeltaSeconds) ; This node is disabled and will not be called.\nDrag off pins to build functionality.
)

(fn ConstructionScript
  (|CallParentFunction))