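; BP_ClusterBombProjectileSmall is a small cluster bomb projectile that explodes on a short fuse timer.
; InitGrenade stores map, manager and owning item, sets damage, levels the spring arm and zeroes X velocity to keep movement in the YZ plane.
; On timeout it stops and hides itself, plays a sound, spawns and initializes a generic explosion actor, then flags itself finished and calls ItemEnd on the owning item.
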(event Custom|InitGrenade
  (params (map :type BP%20Map%20Object%20Reference) (Manager :type BP%20Turn%20Manager%20Object%20Reference) (Owner :type BP%20Item%20Generic%20Object%20Reference))
  (bind _projectilemovement (Variables|Default|GetProjectileMovement))
  (Variables|Default|SetMap map)
  (Variables|Default|SetManager Manager)
  (Variables|Default|SetowningItem Owner)
  (Variables|Default|SetDamage_0 8.0)
  (Transformation|SetWorldRotation (Variables|Default|GetSpringArm) "0, 0, 0" false false)
  (Variables|/Script/Engine.MovementComponent|SetVelocity _projectilemovement (Math|Vector|MakeVector 0.0 (.y (Variables|/Script/Engine.MovementComponent|GetVelocity _projectilemovement)) (.z (Variables|/Script/Engine.MovementComponent|GetVelocity _projectilemovement))))
  (Utilities|Time|SetTimerbyEvent (delegate Custom|GrenadeExplode) 0.25))

(event Custom|GrenadeExplode
  (bind _returnvalue (Transformation|GetActorLocation))
  (bind _sphere (Variables|Default|GetSphere))
  (Components|Activation|Deactivate (Variables|Default|GetProjectileMovement))
  (Components|Tick|SetComponentTickEnabled _sphere false)
  (Collision|SetCollisionEnabled _sphere "NoCollision")
  (Development|SetHiddeninGame _sphere true true)
  (Audio|PlaySoundatLocation "/Game/SFX/SFX_Explosion.SFX_Explosion" _returnvalue "0, 0, 0" 1.0 1.0 0.0 0 0 0 0)
  (bind _returnvalue_2 (Game|SpawnActorfromClass "/Game/WeaponsItems/Generics/BP_ExplsoionGeneric.BP_ExplsoionGeneric_C" (Math|Transform|MakeTransform _returnvalue "0, 0, 0" "0.000000,0.000000,0.000000") "Undefined" "MultiplyWithRoot" 0 0))
  (Default|Init _returnvalue_2 (Variables|Default|GetSize) (Variables|Default|GetMap) (Variables|Default|GetForce) _returnvalue (Variables|Default|GetDamage_0))
  (Variables|Default|SetFinished true)
  (Default|ItemEnd (Variables|Default|GetowningItem)))

(event EventBeginPlay
  (|CallParentFunction) ; This node is disabled and will not be called.\nDrag off pins to build functionality.
)

(event Collision|EventActorBeginOverlap
  (params (OtherActor :type Actor%20Object%20Reference))
  (|CallParentFunction OtherActor) ; This node is disabled and will not be called.\nDrag off pins to build functionality.
)

(event EventTick
  (params (DeltaSeconds :type Float%20%28single-precision%29))
  (|CallParentFunction DeltaSeconds) ; This node is disabled and will not be called.\nDrag off pins to build functionality.
)

(fn ConstructionScript
  (|CallParentFunction))