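; Cluster bomb projectile that explodes on a timer and scatters smaller bomblets.
; InitGrenade stores the map, manager and owning item, sets damage and starts the fuse.
; On expiry it disables movement and collision, hides itself, plays a sound and spawns a generic explosion initialized with map, size, force and damage.
; It then spawns small cluster projectiles at random offsets and orientations, initializing and registering each with the manager.
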(event Custom|InitGrenade
  (params (map :type BP%20Map%20Object%20Reference) (Manager :type BP%20Turn%20Manager%20Object%20Reference) (Owner :type BP%20Item%20Generic%20Object%20Reference))
  (Variables|Default|SetMap map)
  (Variables|Default|SetManager Manager)
  (Variables|Default|SetowningItem Owner)
  (Variables|Default|SetDamage_0 25.0)
  (Transformation|SetWorldRotation (Variables|Default|GetSpringArm) "0, 0, 0" false false)
  (Utilities|Time|SetTimerbyEvent (delegate Custom|GrenadeExplode) 5.0))

(event Custom|GrenadeExplode
  (bind _returnvalue (Transformation|GetActorLocation))
  (bind _sphere (Variables|Default|GetSphere))
  (Components|Activation|Deactivate (Variables|Default|GetProjectileMovement))
  (Components|Tick|SetComponentTickEnabled _sphere false)
  (Collision|SetCollisionEnabled _sphere "NoCollision")
  (Development|SetHiddeninGame _sphere true true)
  (Audio|PlaySoundatLocation "/Game/SFX/SFX_Explosion.SFX_Explosion" _returnvalue "0, 0, 0" 1.0 1.0 0.0 0 0 0 0)
  (bind _returnvalue_2 (Game|SpawnActorfromClass "/Game/WeaponsItems/Generics/BP_ExplsoionGeneric.BP_ExplsoionGeneric_C" (Math|Transform|MakeTransform _returnvalue "0, 0, 0" "0.000000,0.000000,0.000000") "Undefined" "MultiplyWithRoot" 0 0))
  (Default|Init _returnvalue_2 (Variables|Default|GetSize) (Variables|Default|GetMap) (Variables|Default|GetForce) _returnvalue (Variables|Default|GetDamage_0))
  (Variables|Default|SetFinished true)
  (for _index (range 0 9)
    (bind _returnvalue_3 (Game|SpawnActorfromClass "/Game/WeaponsItems/ClusterBomb/BP_ClusterBombProjectileSmall.BP_ClusterBombProjectileSmall_C" (Math|Transform|MakeTransform (+ (* (Math|Random|RandomUnitVector) 1e+02) (Transformation|GetActorLocation self)) (Math|Conversions|RotationFromXVector (Math|Random|RandomUnitVector)) "1.000000,1.000000,1.000000") "AlwaysSpawn" "MultiplyWithRoot" 0 0))
    (Default|InitGrenade _returnvalue_3 (Variables|Default|GetMap) (Variables|Default|GetManager) (Variables|Default|GetowningItem))
    (Default|CreateProjectile (Variables|Default|GetManager) _returnvalue_3)))

(event EventBeginPlay
  (|CallParentFunction) ; This node is disabled and will not be called.\nDrag off pins to build functionality.
)

(event Collision|EventActorBeginOverlap
  (params (OtherActor :type Actor%20Object%20Reference))
  (|CallParentFunction OtherActor) ; This node is disabled and will not be called.\nDrag off pins to build functionality.
)

(event EventTick
  (params (DeltaSeconds :type Float%20%28single-precision%29))
  (|CallParentFunction DeltaSeconds) ; This node is disabled and will not be called.\nDrag off pins to build functionality.
)

(fn ConstructionScript
  (|CallParentFunction))