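; BP_TerrainBombItem is a usable item that launches a terrain bomb projectile for the player who uses it.
; UseItem plays the launch sound, then spawns BP_TerrainBombProjectile offset from the user along the Target vector and facing that direction.
; It initializes the projectile with the map, manager, item and player, and registers it with the manager.
; The user's turn then ends and the first player controller's view blends to follow the projectile.
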(event EventBeginPlay
  (|CallParentFunction) ; This node is disabled and will not be called.\nDrag off pins to build functionality.
)

(event Collision|EventActorBeginOverlap
  (params (OtherActor :type Actor%20Object%20Reference))
  (|CallParentFunction OtherActor) ; This node is disabled and will not be called.\nDrag off pins to build functionality.
)

(event EventTick
  (params (DeltaSeconds :type Float%20%28single-precision%29))
  (|CallParentFunction DeltaSeconds) ; This node is disabled and will not be called.\nDrag off pins to build functionality.
)

(event EventUseItem
  (params (Owner :type BP%20Character%20Object%20Reference) (Target :type Vector :default "0, 0, 0") (Map :type BP%20Map%20Object%20Reference) (Manager :type BP%20Turn%20Manager%20Object%20Reference) (teammates :type Array%20of%20BP%20Character%20Object%20References))
  (Variables|Default|SetOwner_0 Owner)
  (Variables|Default|SetTarget Target)
  (Variables|Default|SetMap Map)
  (Variables|Default|SetManager Manager)
  (Audio|PlaySoundatLocation "/Game/SFX/SFX_Launch.SFX_Launch" (Transformation|GetActorLocation (Variables|Default|GetOwner_0)) "0, 0, 0" 1.0 1.0 0.0 0 0 0 0)
  (bind _returnvalue (Game|SpawnActorfromClass "/Game/WeaponsItems/TerrainBomb/BP_TerrainBombProjectile.BP_TerrainBombProjectile_C" (Math|Transform|MakeTransform (+ (* (Variables|Default|GetTarget) 100) (Transformation|GetActorLocation (Variables|Default|GetOwner_0))) (Math|Conversions|RotationFromXVector (Variables|Default|GetTarget)) "1.000000,1.000000,1.000000") "Undefined" "MultiplyWithRoot" (Variables|Default|GetOwner_0) 0))
  (Default|InitMissile _returnvalue (Variables|Default|GetMap) (Variables|Default|GetManager) self (Variables|Default|GetOwner_0))
  (Default|CreateProjectile (Variables|Default|GetManager) _returnvalue)
  (Default|EndTurn (Variables|Default|GetOwner_0))
  (Game|Player|SetViewTargetwithBlend (Game|GetPlayerController 0) _returnvalue 0.5 "VTBlend_Linear" 0.0 false))

(fn ConstructionScript
  (|CallParentFunction))