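; Projectile for the terrain bomb weapon that explodes on impact and then tells its owning item that its use has ended.
; InitMissile stores map, turn manager, owner and player references, sets damage and briefly ignores collision with the firing player.
; On hit, the sphere is disabled and hidden, and a generic explosion is spawned with the map, size, force and damage, plus a sound.
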(event OnComponentHit(Sphere)
  (params (HitComponent :type Primitive%20Component%20Object%20Reference) (OtherActor :type Actor%20Object%20Reference) (OtherComp :type Primitive%20Component%20Object%20Reference) (NormalImpulse :type Vector :default "0, 0, 0") (Hit :type Hit%20Result%20Structure%20%28by%20ref%29))
  (bind _impactpoint (Collision|BreakHitResult Hit))
  (bind _sphere (Variables|Default|GetSphere))
  (Components|Tick|SetComponentTickEnabled _sphere false)
  (Collision|SetCollisionEnabled _sphere "NoCollision")
  (Development|SetHiddeninGame _sphere true true)
  (bind _returnvalue (Game|SpawnActorfromClass "/Game/WeaponsItems/Generics/BP_ExplsoionGeneric.BP_ExplsoionGeneric_C" (Math|Transform|MakeTransform _impactpoint "0, 0, 0" "0.000000,0.000000,0.000000") "Undefined" "MultiplyWithRoot" 0 0))
  (Default|Init _returnvalue (Variables|Default|GetSize) (Variables|Default|GetMap_0) (Variables|Default|GetForce) _impactpoint (Variables|Default|GetDamage_0))
  (Audio|PlaySoundatLocation "/Game/SFX/SFX_Explosion.SFX_Explosion" _impactpoint "0, 0, 0" 1.0 1.0 0.0 0 0 0 0)
  (Variables|Default|SetFinished true)
  (Default|ItemEnd (Variables|Default|GetOwner_0)))

(event Custom|InitMissile
  (params (map :type BP%20Map%20Object%20Reference) (Manager :type BP%20Turn%20Manager%20Object%20Reference) (Owner :type BP%20Item%20Generic%20Object%20Reference) (Player :type BP%20Character%20Object%20Reference))
  (Variables|Default|SetMap_0 map)
  (Variables|Default|SetTurnManager Manager)
  (Variables|Default|SetOwner_0 Owner)
  (Variables|Default|SetPlayer Player)
  (Variables|Default|SetDamage_0 1e+01)
  (Collision|IgnoreActorwhenMoving (Variables|Default|GetSphere) (Variables|Default|GetPlayer) true)
  (Transformation|SetWorldRotation (Variables|Default|GetSpringArm) "0, 0, 0" false false)
  (Utilities|Time|SetTimerbyEvent (delegate Custom|immunityEnd) 0.2))

(event Custom|immunityEnd
  (Collision|IgnoreActorwhenMoving (Variables|Default|GetSphere) (Variables|Default|GetPlayer) false)
  (Variables|Default|SetinitialImmunity false))

(event EventBeginPlay)

(event Collision|EventActorBeginOverlap
  (params (OtherActor :type Actor%20Object%20Reference)))

(event EventTick
  (params (DeltaSeconds :type Float%20%28single-precision%29)))

(fn ConstructionScript
  (|CallParentFunction))