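; BP_DrillItem is a turn-based weapon item that blasts a line of explosions through whatever lies along the aim direction.
; UseItem line-traces from the owner toward Target in the Y/Z plane, with a fixed end X, and plays an explosion sound.
; It spawns generic explosions interpolated from impact point to trace end, passing each the Map.
; A rifleTimer delay then ends the item and the owner's turn.
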(event Custom|rifleTimer
  (bind _owner_0 (Variables|Default|GetOwner_0))
  (CallFunction|ItemEnd)
  (Utilities|IsValid _owner_0
    (:Is%20Valid
      (Default|EndTurn _owner_0))))

(event EventBeginPlay
  (|CallParentFunction) ; This node is disabled and will not be called.\nDrag off pins to build functionality.
)

(event Collision|EventActorBeginOverlap
  (params (OtherActor :type Actor%20Object%20Reference))
  (|CallParentFunction OtherActor) ; This node is disabled and will not be called.\nDrag off pins to build functionality.
)

(event EventTick
  (params (DeltaSeconds :type Float%20%28single-precision%29))
  (|CallParentFunction DeltaSeconds) ; This node is disabled and will not be called.\nDrag off pins to build functionality.
)

(event EventUseItem
  (params (Owner :type BP%20Character%20Object%20Reference) (Target :type Vector :default "0, 0, 0") (Map :type BP%20Map%20Object%20Reference) (Manager :type BP%20Turn%20Manager%20Object%20Reference) (teammates :type Array%20of%20BP%20Character%20Object%20References))
  (Variables|Default|SetOwner_0 Owner)
  (Variables|Default|SetTarget Target)
  (Variables|Default|SetMap Map)
  (Variables|Default|SetManager Manager)
  (bind _outhit (Collision|LineTraceByChannel (Transformation|GetActorLocation (Variables|Default|GetOwner_0)) (Math|Vector|MakeVector 7.3e+02 (.y (+ (Transformation|GetActorLocation (Variables|Default|GetOwner_0)) (Math|Vector|MakeVector 0.0 (.y (* (Math|Vector|MakeVector 0.0 (.y (Variables|Default|GetTarget)) (.z (Variables|Default|GetTarget))) 1e+03)) (.z (* (Math|Vector|MakeVector 0.0 (.y (Variables|Default|GetTarget)) (.z (Variables|Default|GetTarget))) 1e+03))))) (.z (+ (Transformation|GetActorLocation (Variables|Default|GetOwner_0)) (Math|Vector|MakeVector 0.0 (.y (* (Math|Vector|MakeVector 0.0 (.y (Variables|Default|GetTarget)) (.z (Variables|Default|GetTarget))) 1e+03)) (.z (* (Math|Vector|MakeVector 0.0 (.y (Variables|Default|GetTarget)) (.z (Variables|Default|GetTarget))) 1e+03)))))) "TraceTypeQuery1" true (Utilities|Array|MakeArray (Variables|Default|GetOwner_0)) "None"))
  (Audio|PlaySoundatLocation "/Game/SFX/SFX_Explosion.SFX_Explosion" (Transformation|GetActorLocation (Variables|Default|GetOwner_0)) "0, 0, 0" 1.0 1.0 0.0 0 0 0 0)
  (for _index (range 0 10)
    (bind _returnvalue (Game|SpawnActorfromClass "/Game/WeaponsItems/Generics/BP_ExplsoionGeneric.BP_ExplsoionGeneric_C" (Math|Transform|MakeTransform (Math|Vector|Lerp(Vector) (.impactpoint _outhit) (.traceend _outhit) (/ _index 10)) "0, 0, 0" "1.000000,1.000000,1.000000") "Undefined" "MultiplyWithRoot" 0 0))
    (Default|Init _returnvalue 4.0 (Variables|Default|GetMap) 0.0 (Math|Vector|Lerp(Vector) (.impactpoint _outhit) (.traceend _outhit) (/ _index 10)) 1e+01))
  (Utilities|Time|SetTimerbyEvent (delegate Custom|rifleTimer) 3.0))

(fn ConstructionScript
  (|CallParentFunction))