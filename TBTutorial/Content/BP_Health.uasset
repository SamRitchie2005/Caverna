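; Health component for a BP_Character owner, tracking maximum and current health.
; SetMaxHealth fills health to the given maximum and caches the owning character, while Damage and Heal subtract from or add to current health.
; The CurrentHealth RepNotify handles the consequences, calling Death on the owner at zero or below and otherwise clamping health to the maximum.
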(event Custom|SetMaxHealth
  (params (Maxhealth :type Float%20%28double-precision%29))
  (bind _output_get (Variables|Default|SetMaxHealth Maxhealth))
  (Variables|Default|SetCurrentHealth _output_get)
  (bind _asbp_character (Utilities|Casting|CastToBP_Character (Components|GetOwner)))
  (Variables|Default|SetOwner _asbp_character))

(event Custom|Damage
  (params (Damage :type Float%20%28double-precision%29))
  (Variables|Default|SetCurrentHealth (- (Variables|Default|GetCurrentHealth) Damage)))

(event Custom|Heal
  (params (health :type Float%20%28double-precision%29))
  (Variables|Default|SetCurrentHealth (+ (Variables|Default|GetCurrentHealth) health)))

(event EventTick
  (params (DeltaSeconds :type Float%20%28single-precision%29)))

(fn OnRepCurrentHealth
  (if (<= (Variables|Default|GetCurrentHealth) 0.0)
    (Default|Death (Variables|Default|GetOwner))
    (elif (> (Variables|Default|GetCurrentHealth) (Variables|Default|GetMaxHealth))
      (Variables|Default|SetCurrentHealth (Variables|Default|GetMaxHealth)))))